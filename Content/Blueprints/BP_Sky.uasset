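; BP_Sky is a sky box actor whose appearance follows the rotation of the referenced WorldLight.
; Construction creates a dynamic material on the SkyBox and refreshes it, so the sky also previews in the editor; Tick repeats the update.
; UpdateSky passes the inverted light direction to the material, along with horizon color, zenith color and cloud strength sampled from curves by sun height, a normalized value derived from light pitch.
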(event `self.ReceiveTick`
  (params (DeltaSeconds :type "Float (single-precision)"))
  (`self.UpdateSky`))

(fn `GetSunHeight`
  (returns (ReturnValue :type "Float (double-precision)"))
  (return (`KismetMathLibrary.MapRangeClamped` (.pitch (`self.K2_GetActorRotation` (`self.WorldLight`))) 0.0 -90.0 0.0 1.0)))

(fn `UpdateSky`
  (bind _worldlight (`self.WorldLight`))
  (`/Engine/EditorBlueprintResources/StandardMacros.IsValid` _worldlight
    (:`Is Valid`
      (`MaterialInstanceDynamic.SetVectorParameterValue` (`self.SkyMat`) "LightDirection" (`KismetMathLibrary.Conv_VectorToLinearColor` (* (`SceneComponent.GetForwardVector` (`Actor.RootComponent` _worldlight)) -1.0)))
      (`MaterialInstanceDynamic.SetVectorParameterValue` (`self.SkyMat`) "HorizonColor" (`CurveLinearColor.GetLinearColorValue` (`self.HorizonCurve`) (`self.GetSunHeight`)))
      (`MaterialInstanceDynamic.SetVectorParameterValue` (`self.SkyMat`) "ZenithColor" (`CurveLinearColor.GetLinearColorValue` (`self.ZenithCurve`) (`self.GetSunHeight`)))
      (`MaterialInstanceDynamic.SetScalarParameterValue` (`self.SkyMat`) "CloudStrength" (`CurveFloat.GetFloatValue` (`self.CloudCurve`) (`self.GetSunHeight`))))))

(fn `UserConstructionScript`
  (bind _returnvalue (`KismetMaterialLibrary.CreateDynamicMaterialInstance` (`PrimitiveComponent.GetMaterial` (`self.SkyBox`) 0)))
  (bind _output_get (set `self.SkyMat` _returnvalue))
  (`PrimitiveComponent.SetMaterial` (`self.SkyBox`) 0 _output_get)
  (if (`self.RefreshSky`)
    _
    (else
      _))
  (set `self.RefreshSky` false)
  (`self.UpdateSky`))