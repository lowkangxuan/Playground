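; Solar panel item with a battery that unlocks a button once fully charged; clicking the button destroys the panel.
; The construction script hands CastComponent to the SolarPower component.
; Each tick maps Power charge onto the RingedPowerBar child actor's segments, writing the current segment's fill as instanced-mesh custom data and snapping near-full segments to full.
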(event `self.ReceiveBeginPlay`
  (`ButtonComponent.Enable` (`self.Button`) false))

(event `self.ReceiveTick`
  (params (DeltaSeconds :type "Float (single-precision)"))
  (bind _power (`self.Power`))
  (bind _batteryindicator (`self.BatteryIndicator`))
  (bind _currentpower (`PowerComponent.CurrentPower` _power))
  (bind (_sourcemat _inactivemat _offmat _ringcount _row) (defaults `Object` (castclass `RingedPowerBar` (`ChildActorComponent.ChildActorClass` _batteryindicator) :!pure true)))
  (bind _returnvalue (/ (`PowerComponent.MaxCapacity` _power) (* _ringcount _row)))
  (bind _returnvalue_2 (/ (mod _currentpower _returnvalue) _returnvalue))
  (`InstancedStaticMeshComponent.SetCustomDataValue` (`|GetArrayItem` (`self.K2_GetComponentsByClass` (cast `RingedPowerBar` (`ChildActorComponent.ChildActor` _batteryindicator) :!pure true) "/Script/Engine.InstancedStaticMeshComponent") 1) (`KismetMathLibrary.FFloor` (/ _currentpower _returnvalue)) 0 (`KismetMathLibrary.SelectFloat` 1.0 _returnvalue_2 (> _returnvalue_2 0.994)) true))

(event `self.Power.OnFullCharge`
  (`ButtonComponent.Enable` (`self.Button`) true))

(event `self.Button.OnButtonClicked`
  (`self.K2_DestroyActor`))

(fn `UserConstructionScript`
  (set `SolarPowerComponent.CastComponent` (`self.CastComponent`) (`self.SolarPower`)))