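; BP_Light is a clickable light item that switches between lit and unlit looks depending on whether it is picked up.
; On BeginPlay it hides the BulbOff component.
; On mouse click it runs the parent's click handler, then uses IsPickedUp to show BulbOff when picked up, or PointLight and BulbOn otherwise.
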(event `self.ReceiveBeginPlay`
  (`SceneComponent.SetVisibility` (`self.BulbOff`) false false))

(event `CursorInteractionInterface.OnMouseClicked`
  (bind _bispickedup (`self.bIsPickedUp`))
  (`parent.OnMouseClicked`)
  (`SceneComponent.SetVisibility` (`self.PointLight`) (not _bispickedup) false)
  (`SceneComponent.SetVisibility` (`self.BulbOn`) (not _bispickedup) false)
  (`SceneComponent.SetVisibility` (`self.BulbOff`) _bispickedup false))

(fn `UserConstructionScript`)