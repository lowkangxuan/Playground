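; BP_CampFire is a campfire actor with a flickering point light and a smoke trail plane.
; On BeginPlay it yaws the smoke plane once toward the player character and caches the light's starting intensity.
; It also starts a fast looping timer, apparently driving LightFlicker, which uses a FlipFlop to alternate the light between that intensity and a dimmer one.
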(event `self.ReceiveBeginPlay`
  (`|ExecutionSequence`
    (:`then_0`
      (`SceneComponent.K2_SetWorldRotation` (`self.SM_SmokeTrailPlane`) (`KismetMathLibrary.MakeRotator` 0.0 0.0 (.yaw (`KismetMathLibrary.FindLookAtRotation` (`SceneComponent.K2_GetComponentLocation` (`self.SM_SmokeTrailPlane`)) (`self.K2_GetActorLocation` (`GameplayStatics.GetPlayerCharacter` 0))))) false false))
    (:`then_1`
      (set `self.DefaultLightIntensity` (`LightComponentBase.Intensity` (`self.PointLight`)))
      (`KismetSystemLibrary.K2_SetTimerDelegate` (`|CreateDelegate` :!event `LightFlicker`) 0.1 true))))

(event `LightFlicker`
  (bind _defaultlightintensity (`self.DefaultLightIntensity`))
  (bind _isa (`/Engine/EditorBlueprintResources/StandardMacros.FlipFlop`)
    (:`A`
      _)
    (:`B`
      _))
  (`LightComponent.SetIntensity` (`self.PointLight`) (select `bool` _isa :`false` _defaultlightintensity :`true` (- _defaultlightintensity 350.0) :!type "Float (single-precision)")))

(fn `UserConstructionScript`)