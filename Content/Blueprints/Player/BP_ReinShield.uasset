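; BP_ReinShield is a player shield Blueprint that shows accumulated damage as cracks on its mesh.
; On BeginPlay it replaces the static mesh's first material with a dynamic material instance.
; After each parent damage event it sets that material's Crack parameter to the fraction of health lost, computed from ShieldHealth and CachedShieldHealth.
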(event `self.ReceiveBeginPlay`
  (bind _staticmesh (`self.StaticMesh`))
  (`parent.ReceiveBeginPlay`)
  (bind _returnvalue (`KismetMaterialLibrary.CreateDynamicMaterialInstance` (`PrimitiveComponent.GetMaterial` _staticmesh 0)))
  (bind _output_get (set `self.ShieldMaterialInstance` _returnvalue))
  (`PrimitiveComponent.SetMaterial` _staticmesh 0 _output_get))

(event `ShieldInterface.TakeDamge`
  (params (Damage :type "Float (single-precision)") (DamageEvent :type "DamageEvent Structure (by ref)") (EventInstigator :type "Controller Object Reference") (DamageCauser :type "Actor Object Reference"))
  (`parent.TakeDamge` Damage DamageEvent EventInstigator DamageCauser)
  (`MaterialInstanceDynamic.SetScalarParameterValue` (`self.ShieldMaterialInstance`) "Crack" (- 1.0 (/ (`self.ShieldHealth`) (`self.CachedShieldHealth`)))))

(fn `UserConstructionScript`)