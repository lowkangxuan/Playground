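; Player component that drives a held energy shield mesh, raised while the right mouse button is down.
; Init receives the player and shield meshes, hides the shield, and creates blue and red dynamic material instances.
; Tick pins the shield to ShieldSocket and scales it in or out, disabling itself once fully shrunk.
; While active, keys 1–3 set the ShieldHealth material parameter and Tab swaps colors.
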(event `Key|One`
  (params (Key :type "Key Structure"))
  (:`Pressed`
    (if (`self.IsShieldActive`)
      (`MaterialInstanceDynamic.SetScalarParameterValue` (`self.BlueShieldMatInst`) "ShieldHealth" 2.0)
      (`MaterialInstanceDynamic.SetScalarParameterValue` (`self.RedShieldMatInst`) "ShieldHealth" 2.0))))

(event `Key|Two`
  (params (Key :type "Key Structure"))
  (:`Pressed`
    (if (`self.IsShieldActive`)
      (`MaterialInstanceDynamic.SetScalarParameterValue` (`self.BlueShieldMatInst`) "ShieldHealth" 1.0)
      (`MaterialInstanceDynamic.SetScalarParameterValue` (`self.RedShieldMatInst`) "ShieldHealth" 1.0))))

(event `Key|Three`
  (params (Key :type "Key Structure"))
  (:`Pressed`
    (if (`self.IsShieldActive`)
      (`MaterialInstanceDynamic.SetScalarParameterValue` (`self.BlueShieldMatInst`) "ShieldHealth" 0.0)
      (`MaterialInstanceDynamic.SetScalarParameterValue` (`self.RedShieldMatInst`) "ShieldHealth" 0.0))))

(event `Key|Tab`
  (params (Key :type "Key Structure"))
  (:`Pressed`
    (if (`self.IsShieldActive`)
      (bind _isa (`/Engine/EditorBlueprintResources/StandardMacros.FlipFlop`)
        (:`A`
          _)
        (:`B`
          _))
      (`PrimitiveComponent.SetMaterial` (`self.ShieldMesh`) 0 (select `bool` _isa :`false` (`self.BlueShieldMatInst`) :`true` (`self.RedShieldMatInst`))))))

(event `Key|RightMouseButton`
  (params (Key :type "Key Structure"))
  (:`Pressed`
    (set `self.IsShieldActive` true)
    (`self.SetComponentTickEnabled` true))
  (:`Released`
    (set `self.IsShieldActive` false)))

(event `self.ReceiveTick`
  (params (DeltaSeconds :type "Float (single-precision)"))
  (`|ExecutionSequence`
    (:`then_0`
      (`SceneComponent.K2_SetWorldLocation` (`self.ShieldMesh`) (`SceneComponent.GetSocketLocation` (`self.PlayerMesh`) "ShieldSocket") false false))
    (:`then_1`
      (bind _output_get (set `self.ShieldScale` (`KismetMathLibrary.FInterpTo_Constant` (`self.ShieldScale`) (select `bool` (`self.IsShieldActive`) :`true` 1.0) (`GameplayStatics.GetWorldDeltaSeconds`) 7.0)))
      (`SceneComponent.SetWorldScale3D` (`self.ShieldMesh`) (`KismetMathLibrary.Conv_DoubleToVector` _output_get))
      (if (== (`self.ShieldScale`) 0.0)
        (`self.SetComponentTickEnabled` false)))))

(fn `Init`
  (params (PlayerMesh :type "SkeletalMeshComponent Object Reference") (ShieldMesh :type "StaticMeshComponent Object Reference"))
  (set `self.PlayerMesh` PlayerMesh)
  (bind _output_get (set `self.ShieldMesh` ShieldMesh))
  (`SceneComponent.SetWorldScale3D` _output_get (0.0 0.0 0.0))
  (`|ExecutionSequence`
    (:`then_0`
      (bind _returnvalue (`KismetMaterialLibrary.CreateDynamicMaterialInstance` "/Game/Materials/ReinShield/MI_ReinShield_Blue.MI_ReinShield_Blue"))
      (bind _output_get_2 (set `self.BlueShieldMatInst` _returnvalue))
      (`PrimitiveComponent.SetMaterial` (`self.ShieldMesh`) 0 _output_get_2))
    (:`then_1`
      (bind _returnvalue_2 (`KismetMaterialLibrary.CreateDynamicMaterialInstance` "/Game/Materials/ReinShield/MI_ReinShield_Red.MI_ReinShield_Red"))
      (set `self.RedShieldMatInst` _returnvalue_2))))