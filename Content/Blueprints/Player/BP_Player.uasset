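; Player Blueprint that connects the player's vitals and menu inputs to the HUD.
; On BeginPlay it enables cursor click and hover events, sets unpaused game-only input, seeds the main HUD from DamageableComponent's health and armor, and binds to its post-damage delegate.
; Input events open inventory, pause menu and cheat console widgets through the HUD manager, passing InventoryComponent to the inventory.
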(event `self.ReceiveBeginPlay`
  (bind _returnvalue (`GameplayStatics.GetPlayerController` 0))
  (bind _damageablecomponent (`self.DamageableComponent`))
  (bind _mainhud (`HudManager.MainHUD` (`PlaygroundStatics.GetHudManager`)))
  (`|ExecutionSequence`
    (:`then_0`
      (set `PlayerController.bShowMouseCursor` true _returnvalue)
      (set `PlayerController.bEnableClickEvents` true _returnvalue)
      (set `PlayerController.bEnableMouseOverEvents` true _returnvalue)
      (`PlaygroundGameMode.SetInputModeAndPauseState` (`PlaygroundStatics.GetPlaygroundGameMode`) "OnlyGame" false))
    (:`then_1`
      (`PlayerHUD.SetDefultHUDVitals` _mainhud (`DamageableComponent.BaseHealth` _damageablecomponent) (`DamageableComponent.BaseArmor` _damageablecomponent))
      (`PlayerHUD.UpdateHUDVitals` _mainhud (`DamageableComponent.Health` _damageablecomponent) (`DamageableComponent.Armor` _damageablecomponent))
      (add `DamageableComponent.OnPostDamageTakenDelegate` (`self.DamageableComponent`) (`|CreateDelegate` _mainhud :!event `UpdateHUDVitals`)))))

(event `EnhancedInput|/Game/Inputs/IA_Inventory`
  (params (ActionValue :type Boolean) (ElapsedSeconds :type "Float (double-precision)") (TriggeredSeconds :type "Float (double-precision)") (InputAction :type "InputAction Object Reference" :default "/Game/Inputs/IA_Inventory.IA_Inventory"))
  (:`Started`
    (bind _returnvalue (`HudManager.UploadWidget` (`PlaygroundStatics.GetHudManager`) "/Game/UI/Storages/Inventory/WBP_Inventory.WBP_Inventory_C" false true 0.1))
    (`/Game/UI/Storages/Inventory/WBP_Inventory.Init` (cast `/Game/UI/Storages/Inventory/WBP_Inventory` _returnvalue :!pure true) (`self.InventoryComponent`))))

(event `EnhancedInput|/Game/Inputs/IA_Escape`
  (params (ActionValue :type Boolean) (ElapsedSeconds :type "Float (double-precision)") (TriggeredSeconds :type "Float (double-precision)") (InputAction :type "InputAction Object Reference" :default "/Game/Inputs/IA_Escape.IA_Escape"))
  (:`Started`
    (`HudManager.UploadWidget` (`PlaygroundStatics.GetHudManager`) "/Game/UI/PauseMenu/WBP_PauseMenu.WBP_PauseMenu_C" false true 0.1)))

(event `self.ToggleCheatConsole`
  (`HudManager.UploadWidget` (`PlaygroundStatics.GetHudManager`) "/Game/UI/CheatConsole/WBP_CheatConsole.WBP_CheatConsole_C" false false 0.0))

(fn `UserConstructionScript`)