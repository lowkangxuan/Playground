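; TestDeath is a test actor for a Niagara death effect that takes the place of a skeletal mesh.
; On BeginPlay it feeds the SkeletalMesh component into the Niagara system as a user-variable override and sets a MeshType float parameter.
; After a short delay it activates the Niagara component and hides the mesh in game, leaving the particle effect in its place.
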(event `self.ReceiveBeginPlay`
  (`|ExecutionSequence`
    (:`then_0`
      (`NiagaraFunctionLibrary.OverrideSystemUserVariableSkeletalMeshComponent` (`self.Niagara`) "SkeletalMesh" (`self.SkeletalMesh`))
      (`NiagaraComponent.SetVariableFloat` (`self.Niagara`) "MeshType" 1.0))
    (:`then_1`
      (`KismetSystemLibrary.Delay` 1.0)
      (`ActorComponent.Activate` (`self.Niagara`) false)
      (`SceneComponent.SetHiddenInGame` (`self.SkeletalMesh`) true false))))

(fn `UserConstructionScript`)