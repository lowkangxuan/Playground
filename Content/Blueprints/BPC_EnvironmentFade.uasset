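; Actor component that toggles an environment fade effect by animating the Radius scalar in the MPC_EnvFadeParams material parameter collection.
; Pressing Q alternates the target between DesiredRadius and zero, then enables component tick.
; Tick moves Radius toward the target at constant speed and prints the value to screen.
; Tick starts disabled and switches itself off once the target is reached, so it only runs during a transition.
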(event `self.ReceiveBeginPlay`
  (`self.SetComponentTickEnabled` false))

(event `self.ReceiveTick`
  (params (DeltaSeconds :type "Float (single-precision)"))
  (`|ExecutionSequence`
    (:`then_0`
      (bind _returnvalue (`KismetMaterialLibrary.GetScalarParameterValue` "/Game/Materials/EnvFade/MPC_EnvFadeParams.MPC_EnvFadeParams" "Radius"))
      (bind _returnvalue_2 (`KismetMathLibrary.FInterpTo_Constant` _returnvalue (`self.CurrentRadius`) (`GameplayStatics.GetWorldDeltaSeconds`) 300.0))
      (`KismetSystemLibrary.PrintString` (`KismetStringLibrary.Conv_DoubleToString` _returnvalue_2))
      (`KismetMaterialLibrary.SetScalarParameterValue` "/Game/Materials/EnvFade/MPC_EnvFadeParams.MPC_EnvFadeParams" "Radius" _returnvalue_2))
    (:`then_1`
      (`self.SetComponentTickEnabled` (not (== _returnvalue (`self.CurrentRadius`)))))))

(event `Key|Q`
  (params (Key :type "Key Structure"))
  (:`Pressed`
    (`/Engine/EditorBlueprintResources/StandardMacros.FlipFlop`
      (:`A`
        (set `self.CurrentRadius` (`self.DesiredRadius`)))
      (:`B`
        (set `self.CurrentRadius` 0.0)))
    (`self.SetComponentTickEnabled` true)))