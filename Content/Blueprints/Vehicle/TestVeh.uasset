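; TestVeh is a drivable solar-powered test vehicle that player 0 possesses by interacting with its PickableComponent.
; Possession adds the vehicle input context, whose Enhanced Input actions feed throttle, brake, steering and handbrake to the movement component.
; Throttle requires power and discharges the Power component, which SolarPower recharges from sunlight.
; Tick shows charge on a RingedPowerBar child actor, writing the current segment's fill fraction to instanced-mesh custom data.
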(event `self.ReceiveBeginPlay`
  (set `LightReceivingComponent.CastComponent` (`self.CastComponent`) (`self.SolarPower`)))

(event `self.ReceivePossessed`
  (params (NewController :type "Controller Object Reference"))
  (`EnhancedInputSubsystemInterface.AddMappingContext` (pcsubsystem `EnhancedInputLocalPlayerSubsystem` (`PlaygroundStatics.GetPlaygroundPlayerController`)) "/Game/Inputs/IMC_Vehicle_Context.IMC_Vehicle_Context" 3 (struct)))

(event `self.ReceiveTick`
  (params (DeltaSeconds :type "Float (single-precision)"))
  (bind _power (`self.Power`))
  (bind _childactor (`self.ChildActor`))
  (bind _currentpower (`PowerComponent.CurrentPower` _power))
  (bind (_sourcemat _inactivemat _offmat _ringcount _row) (defaults `Object` (castclass `RingedPowerBar` (`ChildActorComponent.ChildActorClass` _childactor) :!pure true)))
  (bind _returnvalue (/ (`PowerComponent.MaxCapacity` _power) (* _ringcount _row)))
  (bind _returnvalue_2 (/ (mod _currentpower _returnvalue) _returnvalue))
  (bind _asringed_power_bar (cast `RingedPowerBar` (`ChildActorComponent.ChildActor` _childactor)))
  (`InstancedStaticMeshComponent.SetCustomDataValue` (`|GetArrayItem` (`self.K2_GetComponentsByClass` _asringed_power_bar "/Script/Engine.InstancedStaticMeshComponent") 1) (`KismetMathLibrary.FFloor` (/ _currentpower _returnvalue)) 0 (`KismetMathLibrary.SelectFloat` 1.0 _returnvalue_2 (> _returnvalue_2 0.994)) true))

(event `EnhancedInput|/Game/Inputs/Vehicle/IA_Throttle`
  (params (ActionValue :type "Float (double-precision)") (ElapsedSeconds :type "Float (double-precision)") (TriggeredSeconds :type "Float (double-precision)") (InputAction :type "InputAction Object Reference" :default "/Game/Inputs/Vehicle/IA_Throttle.IA_Throttle"))
  (:`Triggered`
    (if (not (<= (`PowerComponent.CurrentPower` (`self.Power`)) 0.0))
      (`ChaosVehicleMovementComponent.SetThrottleInput` (`self.VehicleMovementComponent`) ActionValue :!label _label)
      (`PowerComponent.Discharge` (`self.Power`) (`GameplayStatics.GetWorldDeltaSeconds`))))
  (:`Completed`
    (goto _label)))

(event `EnhancedInput|/Game/Inputs/Vehicle/IA_Reverse`
  (params (ActionValue :type "Float (double-precision)") (ElapsedSeconds :type "Float (double-precision)") (TriggeredSeconds :type "Float (double-precision)") (InputAction :type "InputAction Object Reference" :default "/Game/Inputs/Vehicle/IA_Reverse.IA_Reverse"))
  (:`Triggered`
    (`ChaosVehicleMovementComponent.SetBrakeInput` (`self.VehicleMovementComponent`) ActionValue :!label _label_2))
  (:`Completed`
    (goto _label_2)))

(event `EnhancedInput|/Game/Inputs/Vehicle/IA_Steering`
  (params (ActionValue :type "Float (double-precision)") (ElapsedSeconds :type "Float (double-precision)") (TriggeredSeconds :type "Float (double-precision)") (InputAction :type "InputAction Object Reference" :default "/Game/Inputs/Vehicle/IA_Steering.IA_Steering"))
  (:`Triggered`
    (`ChaosVehicleMovementComponent.SetSteeringInput` (`self.VehicleMovementComponent`) ActionValue :!label _label_3))
  (:`Completed`
    (goto _label_3)))

(event `EnhancedInput|/Game/Inputs/Vehicle/IA_HandBrake`
  (params (ActionValue :type Boolean) (ElapsedSeconds :type "Float (double-precision)") (TriggeredSeconds :type "Float (double-precision)") (InputAction :type "InputAction Object Reference" :default "/Game/Inputs/Vehicle/IA_HandBrake.IA_HandBrake"))
  (:`Triggered`
    (`ChaosVehicleMovementComponent.SetHandbrakeInput` (`self.VehicleMovementComponent`) ActionValue :!label _label_4))
  (:`Completed`
    (goto _label_4)))

(event `self.SolarPower.OnSunlightReceivedDelegate`
  (params (Delta :type "Float (single-precision)"))
  (`PowerComponent.Charge` (`self.Power`) Delta))

(event `self.PickableComponent.OnInteractSuccess`
  (`Controller.Possess` (`GameplayStatics.GetPlayerController` 0) self))

(fn `UserConstructionScript`)